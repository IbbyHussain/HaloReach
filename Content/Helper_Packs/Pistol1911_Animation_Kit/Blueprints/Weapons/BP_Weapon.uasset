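; BP_Weapon is a pickup weapon actor that the player can interact with, equip and drop.
; Entering interaction range spawns a screen-space widget component showing the weapon name on the mesh, and leaving destroys it.
; Interacting calls the player's PickUpGun and sets the state to Equipped, while BeginPlay and Drop set Dropped.
; WeaponState toggles mesh physics and collision on mesh and sphere, and WeaponStruct supplies the name and anim class.
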(event EventBeginPlay
  (Private|WeaponState "NewEnumerator0"))

(event EventOnIntRangeExit
  (bind _interactionwidget (Variables|Private|GetInteractionWidget)
    (:then
      (Components|DestroyComponent _interactionwidget))
    (:else)))

(event EventOnIntRange
  (params (Player :type FPS%20Character%20Object%20Reference))
  (Variables|Private|GetInteractionWidget
    (:then)
    (:else
      (bind _returnvalue (UserInterface|CreateWidget "/Game/Helper_Packs/Pistol1911_Animation_Kit/Blueprints/Interaction_I/Interaction_W.Interaction_W_C" (.AsPlayer%20Controller (Utilities|Casting|CastToPlayerController (Pawn|GetController Player))) (Private|GetWeaponName)))
      (bind _returnvalue_2 (AddComponent|AddWidgetComponent false))
      (bind _output_get (Variables|Private|SetInteractionWidget _returnvalue_2))
      (UserInterface|SetWidget _output_get _returnvalue)
      (Class|WidgetComponent|SetWidgetSpace _output_get "Screen")
      (Class|WidgetComponent|SetDrawatDesiredSize _output_get true)
      (Collision|SetCollisionEnabled _output_get "NoCollision")
      (Transformation|AttachComponentToComponent _output_get (Private|GetWeaponNameAttach) "None" "SnapToTarget" "SnapToTarget" "SnapToTarget" true))))

(event EventOnInt
  (params (Player :type FPS%20Character%20Object%20Reference))
  (Default|PickUpGun Player self)
  (Private|WeaponState "NewEnumerator1"))

(fn ConstructionScript
  (Class|SkeletalMeshComponent|SetAnimClass (Variables|Default|GetWeaponMesh) (.animinstance (Variables|Animation|Parameters|GetWeaponStruct))))

(fn GetWeaponName
  (return (.weaponname (Variables|Animation|Parameters|GetWeaponStruct))))

(fn GetWeaponNameAttach
  (return (Variables|Default|GetWeaponMesh)))

(fn WeaponState
  (params (State :type WeaponState%20Enum :default "NewEnumerator0"))
  (bind _weaponmesh (Variables|Default|GetWeaponMesh))
  (bind _weaponmesh_2 (Variables|Default|GetWeaponMesh))
  (bind _output_get (Variables|Private|SetState State))
  (switch Utilities|FlowControl|Switch|SwitchonWeaponState _output_get
    (:NewEnumerator0
      (Collision|SetCollisionProfileName (Variables|Default|GetSphere) "OverlapAllDynamic" true :!class /Script/Engine.PrimitiveComponent)
      (Physics|SetSimulatePhysics _weaponmesh true)
      (Collision|SetCollisionProfileName _weaponmesh "WeaponCollision" true :!class /Script/Engine.PrimitiveComponent))
    (:NewEnumerator1
      (Collision|SetCollisionProfileName (Variables|Default|GetSphere) "NoCollision" false :!class /Script/Engine.PrimitiveComponent)
      (Physics|SetSimulatePhysics _weaponmesh_2 false)
      (Collision|SetCollisionProfileName _weaponmesh_2 "NoCollision" false :!class /Script/Engine.PrimitiveComponent)
      (Transformation|ResetRelativeTransform (Variables|Default|GetWeaponMesh)))))

(fn Drop
  (Private|WeaponState "NewEnumerator0"))