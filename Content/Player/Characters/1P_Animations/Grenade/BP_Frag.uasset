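; BP_Frag is a throwable frag grenade actor for the first-person player.
; On begin play its static mesh has physics simulation off and ignores the Pawn channel.
; The thrown event enables physics, zeroes velocity and applies a velocity-change impulse scaled by ThrowForce along the player camera's forward vector.
; The up-to-forward lerp is fixed at full forward, and the file contains no fuse or explosion logic.
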(event Custom|thrown
  (bind _staticmesh (Variables|Default|GetStaticMesh))
  (bind _player (Variables|Default|GetPlayer))
  (bind _cameracomp (Variables|/Script/HaloReach.C_PlayerCharacter|GetCameraComp _player))
  (bind _returnvalue (Transformation|GetWorldRotation _cameracomp))
  (Physics|SetSimulatePhysics _staticmesh true)
  (Physics|SetPhysicsLinearVelocity _staticmesh "0, 0, 0" false "None")
  (Physics|AddImpulse (Variables|Default|GetStaticMesh) (* (Math|Vector|Lerp(Vector) (Math|Vector|GetUpVector _returnvalue) (Math|Vector|GetForwardVector _returnvalue) 1.0) (Variables|Default|Getthrow%20force)) "None" true))

(event EventBeginPlay
  (bind _staticmesh (Variables|Default|GetStaticMesh))
  (Physics|SetSimulatePhysics _staticmesh false)
  (Collision|SetCollisionResponsetoChannel _staticmesh "ECC_Pawn" "ECR_Ignore"))

(fn ConstructionScript)