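; Multiplayer player character Blueprint that handles radar icons, death and killer-name tracking.
; BeginPlay gives the locally controlled player an ally icon and others an enemy icon.
; Death multicasts icon removal, flagging the local controller so RefreshIcons can re-add all icons, and sets a RepNotify bool that disables third-person mesh collision.
; AnyDamage passes the damage causer's displayed name to a client check; a name-refresh chain is unconnected.
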(event Custom|Refresh%20Icons
  ;[1 1 1] Adds poi to respawned player
  (bind _asbp_player_controller (Utilities|Casting|CastToBP_PlayerController (Game|GetPlayerController 0)))
  (if (Variables|/Game/Player/BP_PlayerController.BP_PlayerController_C|GetbNewRespawn _asbp_player_controller)
    (bind _outactors (Actor|GetAllActorsOfClass "BP_PlayerCharacter_C"))
    (for _array_element _outactors
      (Class|CRadarIconComponent|AddRadarIcon (Variables|BP_PlayerCharacter_C|GetBP_RadarComponent _array_element))
      (bind _asbp_player_controller_2 (Utilities|Casting|CastToBP_PlayerController (Game|GetPlayerController 0)))
      (Variables|/Game/Player/BP_PlayerController.BP_PlayerController_C|SetbNewRespawn _asbp_player_controller_2 false))))

(event Custom|server
  (params (bool%20brep :type Boolean))
  ;[1 1 1] allows collision to be changed and replicated
  (Variables|Default|Setbool%20brep bool%20brep))

(event Custom|Multi_RemoveRadar
  ;[1 1 1] logic of remove radar icon
  (bind _radaricon (Variables|/Script/HaloReach.C_RadarIconComponent|GetRadarIcon (Variables|Default|GetBP_RadarComponent))
    (:then
      (Widget|RemovefromParent _radaricon)
      (bind _asbp_player_controller (Utilities|Casting|CastToBP_PlayerController (Game|GetPlayerController 0)))
      (Variables|/Game/Player/BP_PlayerController.BP_PlayerController_C|SetbNewRespawn _asbp_player_controller true))
    (:else)))

(event Custom|Remove%20Radar%20Icon
  ;[1 1 1] logic of remove radar icon
  (Networking|SwitchHasAuthority
    (:Authority
      (CallFunction|MultiRemoveRadar))
    (:Remote
      (CallFunction|ServerRemoveRadar))))

(event Custom|Server_RemoveRadar
  ;[1 1 1] logic of remove radar icon
  (CallFunction|MultiRemoveRadar))

(event EventBPDeath
  (params (PlayerKiller :type Actor%20Object%20Reference))
  (Development|PrintString "Player DIED")
  ;[1 1 1] Remove radar icon
  (CallFunction|RemoveRadarIcon)
  ;[1 1 1] allows collision to be changed and replicated
  (if (Ability|HasAuthority)
    (Variables|Default|Setbool%20brep true)
    (else
      (CallFunction|Server true))))

(event EventBeginPlay
  (bind _bp_radarcomponent (Variables|Default|GetBP_RadarComponent))
  (if (Ability|HasAuthority)
    ;[1 1 1] need for server after respawn
    (Utilities|FlowControl|Delay 0.2))
  (Variables|/Script/HaloReach.C_RadarIconComponent|SetOwner _bp_radarcomponent self)
  (if (Pawn|IsLocallyControlled)
    (Variables|/Script/HaloReach.C_RadarIconComponent|SetRadarIconImage _bp_radarcomponent "/Game/UI/Radar/RadarIcons/T_AllyIcon.T_AllyIcon")
    (else
      (Variables|/Script/HaloReach.C_RadarIconComponent|SetRadarIconImage _bp_radarcomponent "/Game/UI/Radar/RadarIcons/T_EnemyIcon.T_EnemyIcon"))))

(event Game|Damage|EventAnyDamage
  (params (Damage :type Float%20%28single-precision%29) (DamageType :type Damage%20Type%20Object%20Reference) (InstigatedBy :type Controller%20Object%20Reference) (DamageCauser :type Actor%20Object%20Reference))
  ;[1 1 1] Successfully updates the player who killed this - not great solution as some weapons do more than 15 dmg
  (Utilities|IsValid DamageCauser
    (:Is%20Valid
      (bind _asbp_player_character (Utilities|Casting|CastToBP_PlayerCharacter DamageCauser))
      (bind _aswbp_player_name (Utilities|Casting|CastToWBP_PlayerName (UserInterface|GetUserWidgetObject (Variables|/Script/HaloReach.C_PlayerCharacter|GetPlayerNameWidgetComp _asbp_player_character))))
      (Class|CPlayerCharacter|ClientCheckKillerName (Variables|/Script/HaloReach.C_PlayerNameWidget|GetDisplayedPlayerName _aswbp_player_name)))))

(fn ConstructionScript)

(fn OnRepBoolBrep
  (Collision|SetCollisionEnabled (Variables|Default|GetMesh3P) "NoCollision")
  (Development|PrintString "on rep"))