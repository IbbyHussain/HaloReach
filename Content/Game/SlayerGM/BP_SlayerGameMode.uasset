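; BP_SlayerGameMode is the Slayer game mode that gives each joining player a randomized team.
; BeginPlay shuffles an array of team values; its following loop does nothing, as the debug prints are disconnected.
; PostLogin waits briefly, casts the player's state to BP_ReachPlayerstate, increments a running index and sets the team from that array entry.
; Despite its name, RandomInt is a sequential counter, so randomness comes only from the shuffle.
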(event EventBeginPlay
  (bind _array (Variables|Default|GetArray))
  ;[1 1 1] Assigns Random Team for all players who join
  (Utilities|Array|Shuffle _array)
  (for _array_element _array
    _))

(event EventPostLogin
  (params (NewPlayer :type Player%20Controller%20Object%20Reference))
  ;[1 1 1] Assigns Random Team for all players who join
  (Utilities|FlowControl|Delay 0.1)
  (bind _asbp_reach_playerstate (Utilities|Casting|CastToBP_ReachPlayerstate (Variables|/Script/Engine.Controller|GetPlayerState NewPlayer)))
  (Math|Integer|IncrementInt (Variables|Default|GetRandom%20Int)
    (:%20%20
      (Class|CReachPlayerState|SetPlayerTeam _asbp_reach_playerstate (Utilities|Enum|ByteToEnumETeam (Math|Conversions|ToByte(Integer) (Utilities|Array|Get(acopy) (Variables|Default|GetArray) (Variables|Default|GetRandom%20Int))))))))

(fn ConstructionScript)