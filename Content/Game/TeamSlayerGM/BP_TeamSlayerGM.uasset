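; Team Slayer game mode that balances players between Red and Blue teams as they join and leave.
; Shortly after login, it adds the controller to the smaller GameState team array, Red on ties, and sets the team on the ReachPlayerstate.
; Logout removes the controller from its array, but casts to BP_PlayerController whereas login casts to C_ReachPlayerController.
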(event EventOnLogout
  (params (ExitingController :type Controller%20Object%20Reference))
  ;[1 1 1] Team Assignment
  (bind _asbp_team_slayer_game_state (Utilities|Casting|CastToBP_TeamSlayerGameState (Game|GetGameState)))
  (bind _asbp_player_controller (Utilities|Casting|CastToBP_PlayerController ExitingController))
  (if (Utilities|Array|ContainsItem (Variables|/Script/HaloReach.C_TeamSlayerGameStateBase|GetRedTeamArray _asbp_team_slayer_game_state) _asbp_player_controller)
    (Utilities|Array|RemoveItem (Variables|/Script/HaloReach.C_TeamSlayerGameStateBase|GetRedTeamArray _asbp_team_slayer_game_state) _asbp_player_controller)
    (else
      (Utilities|Array|RemoveItem (Variables|/Script/HaloReach.C_TeamSlayerGameStateBase|GetBlueTeamArray _asbp_team_slayer_game_state) _asbp_player_controller))))

(event EventPostLogin
  (params (NewPlayer :type Player%20Controller%20Object%20Reference))
  ;[1 1 1] Team Assignment
  (bind _asbp_team_slayer_game_state (Utilities|Casting|CastToBP_TeamSlayerGameState (Game|GetGameState)))
  (Utilities|FlowControl|Delay 0.1)
  (bind _asc_reach_player_controller (Utilities|Casting|CastToC_ReachPlayerController NewPlayer))
  (if (> (Utilities|Array|Length (Variables|/Script/HaloReach.C_TeamSlayerGameStateBase|GetRedTeamArray _asbp_team_slayer_game_state)) (Utilities|Array|Length (Variables|/Script/HaloReach.C_TeamSlayerGameStateBase|GetBlueTeamArray _asbp_team_slayer_game_state)))
    (Utilities|Array|AddUnique (Variables|/Script/HaloReach.C_TeamSlayerGameStateBase|GetBlueTeamArray _asbp_team_slayer_game_state) _asc_reach_player_controller)
    (bind _asbp_reach_playerstate (Utilities|Casting|CastToBP_ReachPlayerstate (Variables|/Script/Engine.Controller|GetPlayerState _asc_reach_player_controller)))
    (Class|CReachPlayerState|SetPlayerTeam _asbp_reach_playerstate "BLUE")
    (else
      (Utilities|Array|AddUnique (Variables|/Script/HaloReach.C_TeamSlayerGameStateBase|GetRedTeamArray _asbp_team_slayer_game_state) _asc_reach_player_controller)
      (bind _asbp_reach_playerstate_2 (Utilities|Casting|CastToBP_ReachPlayerstate (Variables|/Script/Engine.Controller|GetPlayerState _asc_reach_player_controller)))
      (Class|CReachPlayerState|SetPlayerTeam _asbp_reach_playerstate_2 "RED"))))

(fn ConstructionScript)