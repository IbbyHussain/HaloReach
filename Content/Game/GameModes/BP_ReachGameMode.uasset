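; BP_ReachGameMode is a game mode that enforces the lobby player cap.
; On PostLogin it kicks the joining player, with an empty reason, if the player count exceeds MaxPlayers.
; OnLogout is empty, and disconnected leftover nodes for removing controllers from player arrays and assigning the red team never run.
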(event EventPostLogin
  (params (NewPlayer :type Player%20Controller%20Object%20Reference))
  ;[1 1 1] Will kick a player if they are able to join with full lobby
  (Utilities|FlowControl|Sequence
    (:then_0
      (bind _returnvalue (Class|GameModeBase|GetNumPlayers))
      (if (> _returnvalue (Variables|Default|GetMaxPlayers))
        (Class|AdvancedSessionsLibrary|KickPlayer NewPlayer)))))

(event EventOnLogout
  (params (ExitingController :type Controller%20Object%20Reference)))

(fn ConstructionScript)