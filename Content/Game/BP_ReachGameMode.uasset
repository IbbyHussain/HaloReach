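; BP_ReachGameMode is a game mode that tracks connected players and enforces the lobby's player cap.
; On PostLogin it kicks a player who pushes the count above MaxPlayers, then adds the controller to its own PlayerArray and to BP_ReachGameState's PlayerControllerArray.
; That registration runs as a separate sequence step, so it follows even a kick.
; On logout it removes the controller from both arrays.
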(event EventPostLogin
  (params (NewPlayer :type Player%20Controller%20Object%20Reference))
  ;[1 1 1] Will kick a player if they are able to join with full lobby
  (Utilities|FlowControl|Sequence
    (:then_0
      (bind _returnvalue (Class|GameModeBase|GetNumPlayers))
      (if (> _returnvalue (Variables|Default|GetMaxPlayers))
        (Class|AdvancedSessionsLibrary|KickPlayer NewPlayer)))
    (:then_1
      (bind _asbp_reach_game_state (Utilities|Casting|CastToBP_ReachGameState (Game|GetGameState)))
      (bind _asbp_player_controller (Utilities|Casting|CastToBP_PlayerController NewPlayer))
      (Utilities|Array|AddUnique (Variables|/Game/Game/BP_ReachGameState.BP_ReachGameState_C|GetPlayer%20Controller%20Array _asbp_reach_game_state) _asbp_player_controller)
      (Utilities|Array|AddUnique (Variables|Default|GetPlayerArray) _asbp_player_controller))))

(event EventOnLogout
  (params (ExitingController :type Controller%20Object%20Reference))
  (bind _asbp_reach_game_state (Utilities|Casting|CastToBP_ReachGameState (Game|GetGameState)))
  (bind _asbp_player_controller (Utilities|Casting|CastToBP_PlayerController ExitingController))
  (Utilities|Array|RemoveItem (Variables|/Game/Game/BP_ReachGameState.BP_ReachGameState_C|GetPlayer%20Controller%20Array _asbp_reach_game_state) _asbp_player_controller)
  (Utilities|Array|RemoveItem (Variables|Default|GetPlayerArray) _asbp_player_controller))

(fn ConstructionScript)