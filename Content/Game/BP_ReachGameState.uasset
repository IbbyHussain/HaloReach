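; BP_ReachGameState is a game state Blueprint with unfinished logic for showing player deaths on every HUD.
; The Iterateplayers event takes two parameters but currently does nothing.
; Two disconnected loops walk PlayerArray from pawn through controller to BP_PlayerHUD and call UpdateDeathWidget, one with the event's parameters and one with placeholder strings.
; Neither loop runs, and the construction script is empty.
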(event Custom|Iterate%20players
  (params (Name%201 :type String) (NewParam2 :type String)))

(fn ConstructionScript)