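; Game instance Blueprint that handles hosting and joining multiplayer sessions through Advanced Sessions nodes.
; HostSession publishes host name, game mode, map name and max players as extra session settings, then opens The_Lab as a listen server on success.
; The supplied map name is only advertised and does not choose the level that loads.
; JoinSession joins a given search result for the first player controller.
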(event Custom|Host%20Session
  (params (Host%20Name :type Text) (Game%20Mode%20Type :type Text) (Map%20Name :type Text) (Max%20Players :type Integer))
  ;[1 1 1] Host session logic
  (|AdvancedSession (Utilities|Array|MakeArray (Class|AdvancedSessionsLibrary|MakeLiteralSessionPropertyString "SNAME" (Utilities|String|ToString(Text) Host%20Name)) (Class|AdvancedSessionsLibrary|MakeLiteralSessionPropertyString "SGAMEMODE" (Utilities|String|ToString(Text) Game%20Mode%20Type)) (Class|AdvancedSessionsLibrary|MakeLiteralSessionPropertyString "SMAPNAME" (Utilities|String|ToString(Text) Map%20Name)) (Class|AdvancedSessionsLibrary|MakeLiteralSessionPropertyInt "SMaxPlayers" Max%20Players)) (Game|GetPlayerController 0) 100 0 false true false true true false false false true
    (:OnSuccess
      (Game|OpenLevel(byName) "The_Lab" true "?listen"))))

(event Custom|Join%20Session
  (params (Session :type Blueprint%20Session%20Result%20Structure))
  ;[1 1 1] Join session logic
  (|JoinSession (Game|GetPlayerController 0) Session))