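; BP_PainVoume is a pain volume that damages the player and carries a radar component.
; When a BP_PlayerCharacter begins overlapping its Box, it applies FloatDMG damage once and prints the name of player 0, regardless of who entered.
; On BeginPlay it registers itself as the radar component's owner and assigns a red AI icon as its radar image.
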(event OnComponentBeginOverlap(Box)
  (params (OverlappedComponent :type Primitive%20Component%20Object%20Reference) (OtherActor :type Actor%20Object%20Reference) (OtherComp :type Primitive%20Component%20Object%20Reference) (OtherBodyIndex :type Integer) (bFromSweep :type Boolean) (SweepResult :type Hit%20Result%20Structure%20%28by%20ref%29))
  (bind _asbp_player_character (Utilities|Casting|CastToBP_PlayerCharacter OtherActor))
  (Game|Damage|ApplyDamage _asbp_player_character (Variables|Default|Getfloat%20DMG) 0 0)
  (Development|PrintString (PlayerState|GetPlayerName (Variables|/Script/Engine.Controller|GetPlayerState (Game|GetPlayerController 0)))))

(event EventBeginPlay
  (bind _bp_radarcomponent (Variables|Default|GetBP_RadarComponent))
  (Variables|/Script/HaloReach.C_RadarIconComponent|SetOwner _bp_radarcomponent self)
  (Variables|/Script/HaloReach.C_RadarIconComponent|SetRadarIconImage _bp_radarcomponent "/Engine/EngineResources/AICON-Red.AICON-Red"))

(fn ConstructionScript)